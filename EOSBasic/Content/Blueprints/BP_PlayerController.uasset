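; Player controller that exercises an Epic Online Services integration, creating instruction, user info and lobby widgets and initializing the SDK on BeginPlay.
; Input actions trigger DevTool login, logout, Connect login, metrics sessions, user info queries and SDK shutdown, mostly reporting through PrintString.
; Login starts a callback chain that merges friend names, then presence, into the Friends list before subscribing to updates.
; A flag separates the player's own name query from friend lookups.
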(event Custom|LoggedIn
  ;[1 1 1] Basic handling of User Login/Logout Attempts. NOTE: You will need to be published on the Epic Store for this to work!
  (Development|PrintString "Login Successful!" true true "(R=0.000000,G=1.000000,B=0.000000,A=1.000000)" 5.0)
  (Default|ShowHideUserInfo (Variables|Default|GetInstructions) true)
  (bind _returnvalue (Class|EOSManager|GetUserInfo))
  (EventDispatchers|AssignOnUserInfoError _returnvalue (delegate Custom|OnUserInfoError))
  (EventDispatchers|AssignOnUserInfoRetreived _returnvalue (delegate Custom|OnUserInfoRetrieved))
  ;[1 1 1] Stuff with friends - which will use UserInfo that is set above. In order for this to work,through Epic Games Store, you will need friends added in the account portal in order to see them!
  (bind _returnvalue_2 (Class|EOSManager|GetFriends))
  (EventDispatchers|AssignOnFriendActionError _returnvalue_2 (delegate Custom|OnFriendActionError))
  (bind _returnvalue_3 (Class|EOSManager|GetPresence))
  (EventDispatchers|AssignOnFriendPresenceQueryComplete _returnvalue_3 (delegate Custom|OnFriendPresenceQueryComplete))
  (bind _returnvalue_4 (Class|EOSManager|GetFriends))
  (Class|EOSFriends|QueryFriends _returnvalue_4) ; Part 1 - Must do QueryFriends before any other friend calls
)

(event Custom|LoggedOut
  ;[1 1 1] Basic handling of User Login/Logout Attempts. NOTE: You will need to be published on the Epic Store for this to work!
  (Development|PrintString "Logout Successful!" true true "(R=0.000000,G=1.000000,B=0.000000,A=1.000000)" 5.0)
  (Default|ShowHideUserInfo (Variables|Default|GetInstructions) false))

(event Custom|OnConnectLoginFail
  ;[1 1 1] Can login with any OSS. Only tested for Steam at the moment.
  (Development|PrintString "Connect Login Fail" true true "(R=1.000000,G=0.144773,B=0.000000,A=1.000000)" 7.0))

(event Custom|OnConnectSuccess
  ;[1 1 1] Can login with any OSS. Only tested for Steam at the moment.
  (Development|PrintString "Connect Success" true true "(R=0.610907,G=1.000000,B=0.000000,A=1.000000)" 7.0))

(event Custom|LoginFail
  (params (Reason :type String))
  ;[1 1 1] Basic handling of User Login/Logout Attempts. NOTE: You will need to be published on the Epic Store for this to work!
  (Development|PrintString (Utilities|String|Append "Login FAILED with reason: " Reason) true true "(R=1.000000,G=0.000000,B=0.000000,A=1.000000)" 5.0)
  (Default|ShowHideUserInfo (Variables|Default|GetInstructions) false))

(event Custom|RequiresMFA
  ;[1 1 1] Basic handling of User Login/Logout Attempts. NOTE: You will need to be published on the Epic Store for this to work!
  (Development|PrintString "Login Requires MFA!" true true "(R=1.000000,G=0.198145,B=0.000000,A=1.000000)" 5.0))

(event Custom|OnFriendPresenceQueryComplete
  (params (CompleteFriendInfo :type BP%20Cross%20Play%20Info%20Structure%20%28by%20ref%29))
  (bind _temppresencestatuses (Variables|Default|GetTempPresenceStatuses))
  (bind _bpcrossplayfriends (Variables|Default|GetBPCrossPlayFriends))
  (switch Utilities|FlowControl|Switch|SwitchonEPresenceStatus (.Presence (Utilities|Struct|BreakBPPresenceInfo (.presence CompleteFriendInfo))) ; TODO - Do something here further if you want with presence status
    (:Offline
      (Variables|Default|SetTempPresenceStatus "OFFLINE"))
    (:Online
      (Variables|Default|SetTempPresenceStatus "ONLINE"))
    (:Away
      (Variables|Default|SetTempPresenceStatus "AWAY"))
    (:ExtendedAway
      (Variables|Default|SetTempPresenceStatus "EXTENDED AWAY"))
    (:DoNotDisturb
      (Variables|Default|SetTempPresenceStatus "DO NOT DISTURB")))
  (Development|PrintString (Utilities|String|Append (Utilities|String|Append (Utilities|String|Append "Name of Friend: " (.displayname CompleteFriendInfo)) " with presence status of: ") (Variables|Default|GetTempPresenceStatus)) true true "(R=0.358465,G=0.653573,B=1.000000,A=1.000000)" 6.0)
  (Utilities|Array|Add _temppresencestatuses (.presence CompleteFriendInfo))
  (bind _returnvalue (Class|EOSManager|GetFriends))
  (bind _returnvalue_2 (Class|EOSFriends|GetFriendsCount _returnvalue))
  (if (== _returnvalue_2 (Utilities|Array|Length _temppresencestatuses))
    (bind _returnvalue_3 (Class|EOSManager|GetFriends))
    (bind _returnvalue_4 (Class|EOSFriends|GetFriendsCount _returnvalue_3))
    (for _index (range 0 (- _returnvalue_4 1))
      (Utilities|Array|Add (Variables|Default|GetBPCrossPlayFriends) (Utilities|Struct|MakeBPCrossPlayInfo (.accountid (Utilities|Array|Get(acopy) (Variables|/Script/UEOS.EOSFriends|GetTempCrossPlayFriends _returnvalue_3) _index)) (.friendshipstatus (Utilities|Array|Get(acopy) (Variables|/Script/UEOS.EOSFriends|GetTempCrossPlayFriends _returnvalue_3) _index)) (.displayname (Utilities|Array|Get(acopy) (Variables|/Script/UEOS.EOSFriends|GetTempCrossPlayFriends _returnvalue_3) _index)) (Utilities|Array|Get(acopy) (Variables|Default|GetTempPresenceStatuses) _index) (.platformtype (Utilities|Array|Get(acopy) (Variables|/Script/UEOS.EOSFriends|GetTempCrossPlayFriends _returnvalue_3) _index)))))
    (bind _returnvalue_5 (Class|EOSManager|GetFriends))
    (Variables|/Script/UEOS.EOSFriends|SetTempCrossPlayFriends _returnvalue_5 _bpcrossplayfriends)
    (Utilities|Array|Clear _bpcrossplayfriends)
    (bind _returnvalue_6 (Class|EOSManager|GetFriends)) ; We now should have ALL the needed friend info - can subscribe to updates now that will recall some of this stuff!
    (if (not (Variables|Default|GetbSubscribedToUpdates))
      (Class|EOSFriends|SubscribetoFriendUpdates _returnvalue_6)
      (Variables|Default|SetbSubscribedToUpdates true))))

(event Custom|OnUserInfoError
  (params (EpicAccountId :type Epic%20Account%20Id%20Structure%20%28by%20ref%29))
  ;[1 1 1] Basic handling of User Login/Logout Attempts. NOTE: You will need to be published on the Epic Store for this to work!
)

(event Custom|StartEOSSDK
  (bind _instructions (Variables|Default|GetInstructions))
  ;[1 1 1] Attempt to Initialize the EOS SDK.  Called immediately when this PC is made
  (bind (_activeeosmanager _returnvalue) (Class|EOSManager|RequestEOSManager))
  (if _returnvalue
    (bind _returnvalue_2 (Class|EOSManager|InitEOS _activeeosmanager))
    (Development|PrintString (Utilities|String|Append "Init Success status: " (Utilities|String|EnumtoString _returnvalue_2)) true true "(R=0.000000,G=0.660000,B=1.000000,A=1.000000)" 1e+01)
    (Default|ShowHideLogin _instructions false)
    (switch Utilities|FlowControl|Switch|SwitchonEEOSResults _returnvalue_2
      (:ER_Success
        (Default|ShowHideLogin _instructions true)))))

(event Custom|OnUserInfoRetrieved
  (params (EpicAccountId :type Epic%20Account%20Id%20Structure%20%28by%20ref%29))
  (bind _bpcrossplayfriends (Variables|Default|GetBPCrossPlayFriends))
  (bind _tempfriendnames (Variables|Default|GetTempFriendNames))
  ;[1 1 1] Basic handling of User Login/Logout Attempts. NOTE: You will need to be published on the Epic Store for this to work!
  (if (Variables|Default|GetbDoingMyNameQuery)
    (Default|SetPlayerName (Variables|Default|GetUserInfo) (Class|EOSUserInfo|GetDisplayName EpicAccountId))
    (Variables|Default|SetbDoingMyNameQuery false) ; Must reset right after so that friends could do their thing
    (else
      (Utilities|Array|Add _tempfriendnames (Class|EOSUserInfo|GetDisplayName (stale Custom|LoggedIn _returnvalue) EpicAccountId))
      (bind _returnvalue (Class|EOSManager|GetFriends))
      (bind _returnvalue_2 (Class|EOSFriends|GetFriendsCount _returnvalue))
      ;[1 1 1] Stuff with friends - which will use UserInfo that is set above. In order for this to work,through Epic Games Store, you will need friends added in the account portal in order to see them!
      (if (== _returnvalue_2 (Utilities|Array|Length _tempfriendnames))
        (bind _returnvalue_3 (Class|EOSManager|GetFriends))
        (bind _returnvalue_4 (Class|EOSFriends|GetFriendsCount _returnvalue_3))
        (for _index (range 0 (- _returnvalue_4 1))
          (Utilities|Array|Add (Variables|Default|GetBPCrossPlayFriends) (Utilities|Struct|MakeBPCrossPlayInfo (.accountid (Utilities|Array|Get(acopy) (Variables|/Script/UEOS.EOSFriends|GetTempCrossPlayFriends _returnvalue_3) _index)) (.friendshipstatus (Utilities|Array|Get(acopy) (Variables|/Script/UEOS.EOSFriends|GetTempCrossPlayFriends _returnvalue_3) _index)) (Utilities|Array|Get(acopy) (Variables|Default|GetTempFriendNames) _index) (.presence (Utilities|Array|Get(acopy) (Variables|/Script/UEOS.EOSFriends|GetTempCrossPlayFriends _returnvalue_3) _index)) (.platformtype (Utilities|Array|Get(acopy) (Variables|/Script/UEOS.EOSFriends|GetTempCrossPlayFriends _returnvalue_3) _index))))
          (Development|PrintString (Utilities|Array|Get(acopy) (Variables|Default|GetTempFriendNames) _index) true true "(R=0.000000,G=0.660000,B=1.000000,A=1.000000)" 5.0)
          (Development|PrintString (Utilities|String|EnumtoString (.friendshipstatus (Utilities|Array|Get(acopy) (Variables|/Script/UEOS.EOSFriends|GetTempCrossPlayFriends _returnvalue_3) _index))) true true "(R=1.000000,G=0.604231,B=0.000000,A=1.000000)" 5.0))
        (bind _returnvalue_5 (Class|EOSManager|GetFriends))
        (Variables|/Script/UEOS.EOSFriends|SetTempCrossPlayFriends _returnvalue_5 _bpcrossplayfriends)
        (Utilities|Array|Clear _bpcrossplayfriends)
        (bind _returnvalue_6 (Class|EOSManager|GetPresence))
        (Class|EOSPresence|QueryFriendsPresenceInfo _returnvalue_6) ; Part 3 of friend sequence
      ))))

(event Custom|OnFriendActionError
  (params (Reason :type String))
  ;[1 1 1] Stuff with friends - which will use UserInfo that is set above. In order for this to work,through Epic Games Store, you will need friends added in the account portal in order to see them!
  (Development|PrintString Reason true true "(R=0.000000,G=0.660000,B=1.000000,A=1.000000)" 5.0))

(event EventBeginPlay
  (bind _self self)
  (Utilities|FlowControl|Sequence
    (:then_0
      (bind _returnvalue (UserInterface|CreateWidget "/Game/Widgets/W_Instructions.W_Instructions_C" _self))
      (bind _output_get (Variables|Default|SetInstructions _returnvalue))
      (UserInterface|Viewport|AddtoViewport _output_get 0))
    (:then_1
      (bind _returnvalue_2 (UserInterface|CreateWidget "/Game/Widgets/W_UserInfo.W_UserInfo_C" _self))
      (bind _output_get_2 (Variables|Default|SetUserInfo _returnvalue_2))
      (UserInterface|Viewport|AddtoViewport _output_get_2 0))
    (:then_2
      (bind _returnvalue_3 (UserInterface|CreateWidget "/Game/Widgets/W_LobbyUser.W_LobbyUser_C"))
      (UserInterface|Viewport|AddtoViewport _returnvalue_3 0)
      (Variables|Default|SetbShowMouseCursor true))
    (:then_3
      (CallFunction|StartEOSSDK))))

(event Input|ActionEvents|InputActionShutdownEOS
  (params (Key :type Key%20Structure :default "None"))
  ;[1 1 1] Attempt to Shutdown the EOS SDK.  You might put this in your Game Instance's "Event Shutdown" so that this can occur before anything else is torn down, destroyed or disconnected.
  (:Released
    (bind (_activeeosmanager _returnvalue) (Class|EOSManager|RequestEOSManager))
    (if _returnvalue
      (bind _returnvalue_2 (Class|EOSManager|ShutdownEOS _activeeosmanager))
      (Development|PrintString (Utilities|String|Append "Shutdown Success?: " (Utilities|String|EnumtoString _returnvalue_2)) true true "(R=0.000000,G=0.660000,B=1.000000,A=1.000000)" 1e+01)
      (Default|ShowHideLogin (Variables|Default|GetInstructions) false))))

(event Input|ActionEvents|InputActionLogin
  (params (Key :type Key%20Structure :default "None"))
  ;[1 1 1] Basic handling of User Login/Logout Attempts. NOTE: You will need to be published on the Epic Store for this to work!
  (:Released
    (if (not (Utilities|Array|IsEmpty (Variables|/Game/Widgets/W_Instructions.W_Instructions_C|GetCredentialName (Variables|Default|GetInstructions))))
      (bind _returnvalue (Class|EOSManager|IsEOSInitialized))
      (if _returnvalue
        (bind _returnvalue_2 (Class|EOSManager|GetAuthentication))
        (EventDispatchers|BindEventtoOnUserLoggedin _returnvalue_2 (delegate Custom|LoggedIn))
        (EventDispatchers|BindEventtoOnUserLoggedOut _returnvalue_2 (delegate Custom|LoggedOut))
        (EventDispatchers|BindEventtoOnUserLoginFail _returnvalue_2 (delegate Custom|LoginFail))
        (EventDispatchers|BindEventtoOnUserLoginRequiresMFA _returnvalue_2 (delegate Custom|RequiresMFA))
        (Class|EOSAuthentication|Login _returnvalue_2 "LM_DevTool" "localhost:12345" (Variables|/Game/Widgets/W_Instructions.W_Instructions_C|GetCredentialName (Variables|Default|GetInstructions)))
        (Development|PrintString "Attempting to Login..." true true "(R=1.000000,G=0.257687,B=0.000000,A=1.000000)" 5.0)
        (Development|PrintString (Class|EOSManager|GetClientId) true true "(R=0.235119,G=1.000000,B=0.000000,A=1.000000)" 5.0)
        (else
          (Development|PrintString "could not log in"))))))

(event Input|ActionEvents|InputActionLogout
  (params (Key :type Key%20Structure :default "None"))
  (:Released
    ;[1 1 1] Basic handling of User Login/Logout Attempts. NOTE: You will need to be published on the Epic Store for this to work!
    (if (not (Utilities|Array|IsEmpty (Variables|/Game/Widgets/W_Instructions.W_Instructions_C|GetCredentialName (Variables|Default|GetInstructions))))
      (bind _returnvalue (Class|EOSManager|IsEOSInitialized))
      (if _returnvalue
        (bind _returnvalue_2 (Class|EOSManager|GetAuthentication))
        (Class|EOSAuthentication|Logout _returnvalue_2)
        (Default|ShowHideUserInfo (Variables|Default|GetInstructions) false)
        (Default|SetPlayerName (Variables|Default|GetUserInfo))))))

(event Input|ActionEvents|InputActionInitMetric
  (params (Key :type Key%20Structure :default "None"))
  ;[1 1 1] Initialize the Metric.
  (:Released
    (if (not (Utilities|Array|IsEmpty (Variables|/Game/Widgets/W_Instructions.W_Instructions_C|GetCredentialName (Variables|Default|GetInstructions))))
      (bind _returnvalue (Class|EOSManager|GetMetrics))
      (bind _returnvalue_2 (Class|EOSMetrics|InitMetric _returnvalue))
      (Development|PrintString (Utilities|String|Append "Init Metric Success?: " (Utilities|String|ToString(Boolean) _returnvalue_2)) true true "(R=1.000000,G=0.872746,B=0.000000,A=1.000000)" 1e+01))))

(event Input|ActionEvents|InputActionBeginMetricSession
  (params (Key :type Key%20Structure :default "None"))
  ;[1 1 1] Start a Player Session (Display Name is mandatory!)
  (:Released
    (if (not (Utilities|Array|IsEmpty (Variables|/Game/Widgets/W_Instructions.W_Instructions_C|GetCredentialName (Variables|Default|GetInstructions))))
      (bind _returnvalue (Class|EOSManager|GetMetrics))
      (bind _returnvalue_2 (Class|EOSMetrics|BeginPlayerSession _returnvalue "Test" "SAT_External" "ICT_MouseKeyboard"))
      (Development|PrintString (Utilities|String|Append "Begin Player Session?: " (Utilities|String|ToString(Boolean) _returnvalue_2)) true true "(R=0.039068,G=0.359375,B=0.000000,A=1.000000)" 1e+01))))

(event Input|ActionEvents|InputActionEndMetricSession
  (params (Key :type Key%20Structure :default "None"))
  ;[1 1 1] End a Player Session (Display Name should match the one used in Begin)
  (:Released
    (if (not (Utilities|Array|IsEmpty (Variables|/Game/Widgets/W_Instructions.W_Instructions_C|GetCredentialName (Variables|Default|GetInstructions))))
      (bind _returnvalue (Class|EOSManager|GetMetrics))
      (bind _returnvalue_2 (Class|EOSMetrics|EndPlayerSession _returnvalue "Test"))
      (Development|PrintString (Utilities|String|Append "End Player Session?: " (Utilities|String|ToString(Boolean) _returnvalue_2)) true true "(R=0.039068,G=0.359375,B=0.000000,A=1.000000)" 1e+01))))

(event Input|ActionEvents|InputActionGetUserInfo
  (params (Key :type Key%20Structure :default "None"))
  ;[1 1 1] Personal account info
  (:Released
    (if (not (Utilities|Array|IsEmpty (Variables|/Game/Widgets/W_Instructions.W_Instructions_C|GetCredentialName (Variables|Default|GetInstructions))))
      (bind _returnvalue (Class|EOSManager|IsEOSInitialized))
      (if _returnvalue
        (bind _returnvalue_2 (Class|EOSManager|GetAuthentication))
        (bind _returnvalue_3 (Class|EOSManager|GetUserInfo))
        (Variables|Default|SetbDoingMyNameQuery true)
        (Class|EOSUserInfo|QueryUserInfobyAccountId _returnvalue_3 (Class|EOSAuthentication|GetEpicAccountId _returnvalue_2)) ; Callback is set in function call above with SetUser
      ))))

(event Input|ActionEvents|InputActionConnect
  (params (Key :type Key%20Structure :default "None"))
  ;[1 1 1] Can login with any OSS. Only tested for Steam at the moment.
  (:Released
    (if (not (Utilities|Array|IsEmpty (Variables|/Game/Widgets/W_Instructions.W_Instructions_C|GetCredentialName (Variables|Default|GetInstructions))))
      (bind _returnvalue (Class|EOSManager|GetConnect))
      (EventDispatchers|AssignOnConnectLoginFail _returnvalue (delegate Custom|OnConnectLoginFail))
      (EventDispatchers|AssignOnConnectLoginSuccess _returnvalue (delegate Custom|OnConnectSuccess))
      (Class|EOSConnect|Login _returnvalue "ECT_Epic"))))

(fn ConstructionScript)